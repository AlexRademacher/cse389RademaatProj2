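; BP_PlayerCharacter is the player character Blueprint, handling HUD setup and opening the pause menu.
; On BeginPlay it sets game-only input and adds a WBP_HUD widget to the viewport.
; Pressing P lazily creates and caches WBP_Pause, shows it if not already visible, pauses the game and reveals the mouse cursor.
; It contains no unpause logic.
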(event EventBeginPlay
  (Input|SetInputModeGameOnly (Game|GetPlayerController 0) false)
  (bind _returnvalue (UserInterface|CreateWidget "/Game/UI/WBP_HUD.WBP_HUD_C"))
  (UserInterface|Viewport|AddtoViewport _returnvalue 0))

(event Collision|EventActorBeginOverlap
  (params (OtherActor :type Actor%20Object%20Reference)))

(event EventTick
  (params (DeltaSeconds :type Float%20%28single-precision%29)))

(event Input|KeyboardEvents|P
  (params (Key :type Key%20Structure :default "None"))
  (:Pressed
    (Utilities|IsValid (Variables|Default|GetPause%20Reference)
      (:Is%20Valid
        (if (not (Widget|IsVisible (Variables|Default|GetPause%20Reference)))
          (UserInterface|Viewport|AddtoViewport (Variables|Default|GetPause%20Reference) 0 :!label _label)
          (Game|SetGamePaused true)
          (Variables|/Script/Engine.PlayerController|SetbShowMouseCursor (Game|GetPlayerController 0) true)))
      (:Is%20Not%20Valid
        (bind _returnvalue (UserInterface|CreateWidget "/Game/UI/WBP_Pause.WBP_Pause_C"))
        (Variables|Default|SetPause%20Reference _returnvalue)
        (goto _label)))))

(fn ConstructionScript)